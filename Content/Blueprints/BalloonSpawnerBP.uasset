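; Balloon spawner actor that continuously spawns BadBalloonBP actors around its own position.
; From BeginPlay it loops forever: spawn a balloon, wait DelayTime, then repeat.
; Each spawn lands at a random X/Y offset within SpawnRadius on both axes, forming a square area, at the spawner's height with zero rotation.
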(event `self.ReceiveBeginPlay`
  (bind _spawnradius (`self.SpawnRadius`))
  (bind _returnvalue (* _spawnradius -1.0))
  (`|SpawnActorFromClass` "/Game/Blueprints/BadBalloonBP.BadBalloonBP_C" (`KismetMathLibrary.MakeTransform` (`KismetMathLibrary.MakeVector` (+ (.x (`self.K2_GetActorLocation`)) (`KismetMathLibrary.RandomFloatInRange` _returnvalue _spawnradius)) (+ (.y (`self.K2_GetActorLocation`)) (`KismetMathLibrary.RandomFloatInRange` _returnvalue _spawnradius)) (.z (`self.K2_GetActorLocation`)))) "Undefined" "OverrideRootScale" null null :!label _label)
  (`KismetSystemLibrary.Delay` (`self.DelayTime`))
  (goto _label))

(fn `UserConstructionScript`)